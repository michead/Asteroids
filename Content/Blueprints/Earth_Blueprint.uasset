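; Earth actor that spawns incoming debug targets and launches rockets at them.
; From BeginPlay it enables input and loops every two seconds, spawning a Debug_target at a random point on the XZ plane with a reference to itself.
; Pressing R spawns a Rocket at Earth aimed at the most recently spawned target.
; Overlapping a Debug_target plays a fire emitter at Earth and destroys that target.
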(event EventBeginPlay
  ;[1 1 1] enable input
  (Input|EnableInput (Game|GetPlayerController 0))
  ;[1 1 1] foes creation
  (bind _output_get (Variables|Default|Settarget_location (Math|Vector|MakeVector (Math|Random|RandomFloatinRange -5e+02 5e+02) 0.0 (Math|Random|RandomFloatinRange -5e+02 5e+02)) :!label _label))
  ;;[1 1 1] create dedug target
  (bind _returnvalue (Game|SpawnActorfromClass "/Game/Blueprints/debug_target.debug_target_C" (Math|Conversions|ToTransform(Vector) _output_get) false self 0))
  (Utilities|FlowControl|Delay 2.0)
  (goto _label))

(event EventActorBeginOverlap
  (params (OtherActor :type Actor%20Object%20Reference))
  ;[1 1 1] collision with asteroids
  (if (== (Utilities|GetClass OtherActor) "/Game/Blueprints/debug_target.debug_target_C")
    (Effects|SpawnEmitteratLocation "/Game/StarterContent/Particles/P_Fire.P_Fire" (Transformation|GetActorLocation) "0,0.000000, 0")
    (Actor|DestroyActor OtherActor)))

(event Input|KeyboardEvents|R
  ;[1 1 1] right word commit
  (:Pressed
    ;[1 1 1] spawn rocket
    (Game|SpawnActorfromClass "/Game/Blueprints/rocket.rocket_C" (Transformation|GetActorTransform) false 3e+01 (stale EventBeginPlay _returnvalue) 0)))

(fn ConstructionScript)