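; Word-labeled asteroid actor that takes as many missile hits to destroy as its word has letters.
; Construction randomizes angular velocity and places the word text at the bounds' Y extent; Tick applies only the Y component as local pitch spin.
; Missile overlaps decrement health, with the final hit destroying both actors and adding to Earth's score.
; Hitting Earth destroys the asteroid, damages Earth and also refreshes the score display.
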(event EventBeginPlay
  (Variables|Default|SetHealth (Utilities|String|Len (Variables|Default|GetWord)))
  (bind _outactors (Actor|GetAllActorsOfClass "/Game/Blueprints/Earth.Earth_C"))
  (Variables|Default|SetEarth (Utilities|Array|Get(acopy) _outactors)))

(event EventTick
  (params (DeltaSeconds :type Float%20%28single-precision%29))
  (Transformation|AddActorLocalRotation (Class|KismetMathLibrary|MakeRot (.Y (Math|Vector|BreakVector (* (Variables|Default|GetAngularVelocity) DeltaSeconds))) 0.0 0.0) false))

(event EventActorBeginOverlap
  (params (OtherActor :type Actor%20Object%20Reference))
  (bind _earth (Variables|Default|GetEarth))
  (bind _asmissile (Utilities|Casting|CastToMissile OtherActor)
    (:then
      (Variables|Default|SetHealth (- (Variables|Default|GetHealth) 1))
      (if (== (Variables|Default|GetHealth) 0)
        (Actor|DestroyActor)
        (Actor|DestroyActor _asmissile)
        (Variables|/Game/Blueprints/Earth.Earth_C|SetScore _earth (+ (Variables|/Game/Blueprints/Earth.Earth_C|GetScore _earth) (Variables|Default|GetDeltaScoreOnDestroy)))
        (Default|UpdatePlayerScore _earth :!label _label)
        (Variables|Default|SetWord (Utilities|String|GetSubstring (Variables|Default|GetWord) 0 (Utilities|String|Len (Variables|Default|GetWord))))))
    (:CastFailed
      (Utilities|Casting|CastToEarth OtherActor)
      (Actor|DestroyActor)
      (Variables|/Game/Blueprints/Earth.Earth_C|SetHealth _earth (- (Variables|/Game/Blueprints/Earth.Earth_C|GetHealth _earth) (Variables|Default|GetDamageOnHit)))
      (goto _label))))

(fn ConstructionScript
  (bind _spinningword (Variables|Default|GetSpinningWord))
  (bind _minrot (Variables|Default|GetMinRot))
  (bind _maxrot (Variables|Default|GetMaxRot))
  (Variables|Default|SetAngularVelocity (Math|Vector|MakeVector (Math|Random|RandomFloatinRange _minrot _maxrot) (Math|Random|RandomFloatinRange _minrot _maxrot) (Math|Random|RandomFloatinRange _minrot _maxrot)))
  (Rendering|Components|TextRender|SetText _spinningword (Variables|Default|GetWord))
  (Transformation|SetRelativeLocation _spinningword (Math|Vector|MakeVector 0.0 (.Y (Math|Vector|BreakVector (.BoxExtent (Collision|GetActorBounds false)))) 0.0) false))