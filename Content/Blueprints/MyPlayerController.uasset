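; Player controller for a typing game where letter keys lock onto Asteroids by their words and fire rockets from Earth.
; KeyInput's floored axis value indexes an Alphabet array, and that letter is compared with the first character of a Word.
; Unlocked, a matching Asteroid sets TargetLocked but Earth.Target is set to None; locked, a match spawns a rocket and an invalid target releases the lock.
; The construction script caches the first Earth actor.
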(event EventBeginPlay)

(event EventTick
  (params (DeltaSeconds :type Float%20%28single-precision%29)))

(event Input|AxisEvents|InputAxisKeyInput
  (params (AxisValue :type Float%20%28single-precision%29))
  (bind _earth (Variables|Default|GetEarth))
  (if (Variables|Default|GetTargetLocked)
    ;[1 1 1] Spawn rocket
    (if (Utilities|IsValid (Variables|/Game/Blueprints/Earth.Earth_C|GetTarget _earth))
      (if (Utilities|Enum|Equal(Enum) (Utilities|String|GetSubstring (Variables|/Game/Blueprints/Asteroid.Asteroid_C|GetWord (Variables|/Game/Blueprints/Earth.Earth_C|GetTarget _earth)) 0) (Utilities|String|ToString(Text) (Utilities|Array|Get(acopy) (Variables|Default|GetAlphabet) (Math|Float|Floor AxisValue))))
        (Default|SpawnRocket _earth))
      (else
        (Variables|Default|SetTargetLocked false)))
    (else
      ;[1 1 1] Lock target
      (bind _outactors (Actor|GetAllActorsOfClass "/Game/Blueprints/Asteroid.Asteroid_C"))
      (bind _array_element (Utilities|Array|ForEachLoopwithBreak _outactors :!label _label)
        (:LoopBody
          (if (Utilities|Enum|Equal(Enum) (Utilities|String|GetSubstring (Variables|/Game/Blueprints/Asteroid.Asteroid_C|GetWord _array_element) 0) (Utilities|String|ToString(Text) (Utilities|Array|Get(acopy) (Variables|Default|GetAlphabet) (Math|Float|Floor AxisValue))))
            (Variables|/Game/Blueprints/Earth.Earth_C|SetTarget (Variables|Default|GetEarth) 0)
            (Variables|Default|SetTargetLocked true)
            (goto _label Break)))))))

(fn ConstructionScript
  (bind _outactors (Actor|GetAllActorsOfClass "/Game/Blueprints/Earth.Earth_C"))
  (Variables|Default|SetEarth (Utilities|Array|Get(acopy) _outactors)))